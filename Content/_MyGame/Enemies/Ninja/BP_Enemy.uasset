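; Ninja enemy Blueprint that reacts to hits on individual body parts and dies into a ragdoll.
; Overlap events on head, torso front and back, arm and leg hitboxes trigger matching directional hit-reaction functions, ignored once the Health component reports death.
; The Health component's death event triggers the ragdoll, and an Attack event plays the ninja melee montage.
; Debug strings print on each hit and on death.
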(event OnDied(Health)
  (Development|PrintString "Enemy Died" true false "(R=1.000000,G=0.000000,B=0.197663,A=1.000000)")
  (Class|Enemy|DeathRagdoll))

(event OnComponentBeginOverlap(HeadHitBox)
  (params (OverlappedComponent :type Primitive%20Component%20Object%20Reference) (OtherActor :type Actor%20Object%20Reference) (OtherComp :type Primitive%20Component%20Object%20Reference) (OtherBodyIndex :type Integer) (bFromSweep :type Boolean) (SweepResult :type Hit%20Result%20Structure%20%28by%20ref%29))
  (if (not (Class|HealthComponent|GetIsDead (Variables|Default|GetHealth)))
    (Development|PrintString "Enemy HEAD Hit (Overlap)" true false "(R=0.000000,G=1.000000,B=0.892101,A=1.000000)")
    (Class|Enemy|TopHeadHit)))

(event OnComponentBeginOverlap(BodyFrontHitBox)
  (params (OverlappedComponent :type Primitive%20Component%20Object%20Reference) (OtherActor :type Actor%20Object%20Reference) (OtherComp :type Primitive%20Component%20Object%20Reference) (OtherBodyIndex :type Integer) (bFromSweep :type Boolean) (SweepResult :type Hit%20Result%20Structure%20%28by%20ref%29))
  (if (not (Class|HealthComponent|GetIsDead (Variables|Default|GetHealth)))
    (Development|PrintString "Enemy BODY hit" true false)
    (Class|Enemy|FrontStomachHit)))

(event OnComponentBeginOverlap(BodyBackHitBox)
  (params (OverlappedComponent :type Primitive%20Component%20Object%20Reference) (OtherActor :type Actor%20Object%20Reference) (OtherComp :type Primitive%20Component%20Object%20Reference) (OtherBodyIndex :type Integer) (bFromSweep :type Boolean) (SweepResult :type Hit%20Result%20Structure%20%28by%20ref%29))
  (if (not (Class|HealthComponent|GetIsDead (Variables|Default|GetHealth)))
    (Development|PrintString "Enemy Back HIT")
    (Class|Enemy|BackHit)))

(event OnComponentBeginOverlap(LeftLegHitBox)
  (params (OverlappedComponent :type Primitive%20Component%20Object%20Reference) (OtherActor :type Actor%20Object%20Reference) (OtherComp :type Primitive%20Component%20Object%20Reference) (OtherBodyIndex :type Integer) (bFromSweep :type Boolean) (SweepResult :type Hit%20Result%20Structure%20%28by%20ref%29))
  (if (not (Class|HealthComponent|GetIsDead (Variables|Default|GetHealth)))
    (Development|PrintString "Enemy Left Leg HIT")
    (Class|Enemy|LeftLegHit)))

(event OnComponentBeginOverlap(RightLegHitBox)
  (params (OverlappedComponent :type Primitive%20Component%20Object%20Reference) (OtherActor :type Actor%20Object%20Reference) (OtherComp :type Primitive%20Component%20Object%20Reference) (OtherBodyIndex :type Integer) (bFromSweep :type Boolean) (SweepResult :type Hit%20Result%20Structure%20%28by%20ref%29))
  (if (not (Class|HealthComponent|GetIsDead (Variables|Default|GetHealth)))
    (Development|PrintString "Enemy Right Leg HIT")
    (Class|Enemy|RightLegHit)))

(event OnComponentBeginOverlap(LeftLowerArmHitBox)
  (params (OverlappedComponent :type Primitive%20Component%20Object%20Reference) (OtherActor :type Actor%20Object%20Reference) (OtherComp :type Primitive%20Component%20Object%20Reference) (OtherBodyIndex :type Integer) (bFromSweep :type Boolean) (SweepResult :type Hit%20Result%20Structure%20%28by%20ref%29))
  (if (not (Class|HealthComponent|GetIsDead (Variables|Default|GetHealth)))
    (Development|PrintString "Enemy LEFT LOWER ARM hit" true false "(R=0.158250,G=1.000000,B=0.000000,A=1.000000)")
    (Class|Enemy|LeftSideHit)))

(event OnComponentBeginOverlap(RightLowerArmHitBox)
  (params (OverlappedComponent :type Primitive%20Component%20Object%20Reference) (OtherActor :type Actor%20Object%20Reference) (OtherComp :type Primitive%20Component%20Object%20Reference) (OtherBodyIndex :type Integer) (bFromSweep :type Boolean) (SweepResult :type Hit%20Result%20Structure%20%28by%20ref%29))
  (if (not (Class|HealthComponent|GetIsDead (Variables|Default|GetHealth)))
    (Development|PrintString "Enemy RIGHT LOWER ARM hit" true false "(R=0.158250,G=1.000000,B=0.000000,A=1.000000)")
    (Class|Enemy|RightSideHit)))

(event OnComponentBeginOverlap(RightUpperArmHitBox)
  (params (OverlappedComponent :type Primitive%20Component%20Object%20Reference) (OtherActor :type Actor%20Object%20Reference) (OtherComp :type Primitive%20Component%20Object%20Reference) (OtherBodyIndex :type Integer) (bFromSweep :type Boolean) (SweepResult :type Hit%20Result%20Structure%20%28by%20ref%29))
  (if (not (Class|HealthComponent|GetIsDead (Variables|Default|GetHealth)))
    (Development|PrintString "Enemy RIGHT UPPER ARM hit" true false "(R=0.158250,G=1.000000,B=0.000000,A=1.000000)")
    (Class|Enemy|RightSideHit)))

(event Custom|Attack
  (Animation|Montage|PlayMontage (Variables|Character|GetMesh) "/Game/_MyGame/Animation/Enemy/AM_Enemy_NinjaMelee.AM_Enemy_NinjaMelee"))

(event EventBeginPlay)

(event Collision|EventActorBeginOverlap
  (params (OtherActor :type Actor%20Object%20Reference)))

(event EventTick
  (params (DeltaSeconds :type Float%20%28single-precision%29)))

(fn ConstructionScript)