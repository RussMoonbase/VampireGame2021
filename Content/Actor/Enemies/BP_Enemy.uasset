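; BP_Enemy is an enemy that reacts to hits by body region and ragdolls on death.
; Overlaps on the head, right upper arm and body hit boxes each call their own hit reaction, but only while the Health component reports it is alive.
; Health's OnDied event calls DeathRagdoll, and every handler prints a debug message.
; The overlap handlers apply no damage, and the reaction and ragdoll logic is defined outside these graphs.
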(event OnDied(Health)
  (Development|PrintString "Enemy Died" true false "(R=1.000000,G=0.000000,B=0.197663,A=1.000000)")
  (Class|Enemy|DeathRagdoll))

(event OnComponentBeginOverlap(RightUpperArmHitBox)
  (params (OverlappedComponent :type Primitive%20Component%20Object%20Reference) (OtherActor :type Actor%20Object%20Reference) (OtherComp :type Primitive%20Component%20Object%20Reference) (OtherBodyIndex :type Integer) (bFromSweep :type Boolean) (SweepResult :type Hit%20Result%20Structure%20%28by%20ref%29))
  (if (not (Class|HealthComponent|GetIsDead (Variables|Default|GetHealth)))
    (Development|PrintString "Enemy RIGHT UPPER ARM hit" true false "(R=0.158250,G=1.000000,B=0.000000,A=1.000000)")
    (Class|Enemy|RightSideHit)))

(event OnComponentBeginOverlap(HeadHitBox)
  (params (OverlappedComponent :type Primitive%20Component%20Object%20Reference) (OtherActor :type Actor%20Object%20Reference) (OtherComp :type Primitive%20Component%20Object%20Reference) (OtherBodyIndex :type Integer) (bFromSweep :type Boolean) (SweepResult :type Hit%20Result%20Structure%20%28by%20ref%29))
  (if (not (Class|HealthComponent|GetIsDead (Variables|Default|GetHealth)))
    (Development|PrintString "Enemy HEAD Hit (Overlap)" true false "(R=0.000000,G=1.000000,B=0.892101,A=1.000000)")
    (Class|Enemy|TopHeadHit)))

(event OnComponentBeginOverlap(BodyHitBox)
  (params (OverlappedComponent :type Primitive%20Component%20Object%20Reference) (OtherActor :type Actor%20Object%20Reference) (OtherComp :type Primitive%20Component%20Object%20Reference) (OtherBodyIndex :type Integer) (bFromSweep :type Boolean) (SweepResult :type Hit%20Result%20Structure%20%28by%20ref%29))
  (if (not (Class|HealthComponent|GetIsDead (Variables|Default|GetHealth)))
    (Development|PrintString "Enemy BODY hit" true false)
    (Class|Enemy|FrontStomachHit)))

(event EventBeginPlay)

(event Collision|EventActorBeginOverlap
  (params (OtherActor :type Actor%20Object%20Reference)))

(event EventTick
  (params (DeltaSeconds :type Float%20%28single-precision%29)))

(fn ConstructionScript)